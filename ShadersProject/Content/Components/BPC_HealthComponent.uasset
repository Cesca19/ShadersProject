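; Health component that tracks an owner's Health and Dead state.
; TakeDamage subtracts the incoming amount from Health, clamping it to zero and setting Dead when it would reach zero or below.
; Tick polls the Dead flag and calls OnDeath every frame while it is true, with no one-shot guard.
; OnDeath has an empty body, so death has no effect within this component.
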(event `self.ReceiveTick`
  (params (DeltaSeconds :type "Float (single-precision)"))
  (if (`self.Dead`)
    (`self.OnDeath`)))

(fn `OnDeath`)

(fn `TakeDamage`
  (params (B :type Integer))
  (bind _returnvalue (- (`self.Health`) B))
  (if (<= _returnvalue 0)
    (set `self.Health` 0)
    (set `self.Dead` true)
    (else
      (set `self.Health` _returnvalue))))