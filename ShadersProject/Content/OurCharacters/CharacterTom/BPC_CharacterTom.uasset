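; Player character Blueprint for Tom that prototypes a bow shot and a four-stage bow combo through Enhanced Input actions.
; Shoot input is gated by the AttackShoot flag and short delays, though the Shoot function only sets that flag.
; Combo inputs increment ComboState under upper-bound checks and print debug text; cancelling any resets it.
; The BowCombo functions are empty, and the skill input only prints a placeholder string.
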(event `EnhancedInput|/Game/OurCharacters/IA/IA_Skill`
  (params (ActionValue :type Boolean) (ElapsedSeconds :type "Float (double-precision)") (TriggeredSeconds :type "Float (double-precision)") (InputAction :type "InputAction Object Reference" :default "/Game/OurCharacters/IA/IA_Skill.IA_Skill"))
  (:`Triggered`
    (`KismetSystemLibrary.PrintString` "ta mere")))

(event `EnhancedInput|/Game/OurCharacters/IA/IA_Shoot`
  (params (ActionValue :type Boolean) (ElapsedSeconds :type "Float (double-precision)") (TriggeredSeconds :type "Float (double-precision)") (InputAction :type "InputAction Object Reference" :default "/Game/OurCharacters/IA/IA_Shoot.IA_Shoot"))
  (:`Triggered`
    (if (not (`self.AttackShoot`))
      (set `self.CanGoToNextCombo` false)
      (set `self.AttackShoot` true)
      (`KismetSystemLibrary.Delay` 0.226)
      (`self.Shoot`)
      (`KismetSystemLibrary.Delay` 0.15)
      (set `self.AttackShoot` false)
      (if (`self.Combo1Triggered`)
        _))))

(event `EnhancedInput|/Game/OurCharacters/IA/IA_BowCombo1`
  (params (ActionValue :type Boolean) (ElapsedSeconds :type "Float (double-precision)") (TriggeredSeconds :type "Float (double-precision)") (InputAction :type "InputAction Object Reference" :default "/Game/OurCharacters/IA/IA_BowCombo1.IA_BowCombo1"))
  (bind _combo_state (`self.Combo State`))
  (:`Triggered`
    (if (< _combo_state 1)
      (`KismetSystemLibrary.PrintString` "Combo 1")
      (`/Engine/EditorBlueprintResources/StandardMacros.IncrementInt` _combo_state
        (:`  `
          (set `self.Combo1Triggered` true)))))
  (:`Canceled`
    (set `self.Combo State` 0 :!label _label)))

(event `EnhancedInput|/Game/OurCharacters/IA/IA_BowCombo2`
  (params (ActionValue :type Boolean) (ElapsedSeconds :type "Float (double-precision)") (TriggeredSeconds :type "Float (double-precision)") (InputAction :type "InputAction Object Reference" :default "/Game/OurCharacters/IA/IA_BowCombo2.IA_BowCombo2"))
  (bind _combo_state (`self.Combo State`))
  (:`Triggered`
    (if (<= _combo_state 2)
      (`KismetSystemLibrary.PrintString` "Combo 2")
      (`/Engine/EditorBlueprintResources/StandardMacros.IncrementInt` _combo_state)))
  (:`Canceled`
    (goto _label)))

(event `EnhancedInput|/Game/OurCharacters/IA/Ia_BowCombo3`
  (params (ActionValue :type Boolean) (ElapsedSeconds :type "Float (double-precision)") (TriggeredSeconds :type "Float (double-precision)") (InputAction :type "InputAction Object Reference" :default "/Game/OurCharacters/IA/Ia_BowCombo3.Ia_BowCombo3"))
  (bind _combo_state (`self.Combo State`))
  (:`Triggered`
    (if (<= _combo_state 3)
      (`KismetSystemLibrary.PrintString` "Combo 3")
      (`/Engine/EditorBlueprintResources/StandardMacros.IncrementInt` _combo_state)))
  (:`Canceled`
    (goto _label)))

(event `EnhancedInput|/Game/OurCharacters/IA/IA_BowCombo4`
  (params (ActionValue :type Boolean) (ElapsedSeconds :type "Float (double-precision)") (TriggeredSeconds :type "Float (double-precision)") (InputAction :type "InputAction Object Reference" :default "/Game/OurCharacters/IA/IA_BowCombo4.IA_BowCombo4"))
  (bind _combo_state (`self.Combo State`))
  (:`Triggered`
    (if (<= _combo_state 4)
      (`KismetSystemLibrary.PrintString` "Combo 4")
      (`/Engine/EditorBlueprintResources/StandardMacros.IncrementInt` _combo_state)))
  (:`Canceled`
    (goto _label)))

(fn `BowCombo1`)

(fn `BowCombo2`)

(fn `BowCombo3`)

(fn `BowCombo4`)

(fn `Shoot`
  (set `self.AttackShoot` true))

(fn `UserConstructionScript`
  (`parent.UserConstructionScript`))