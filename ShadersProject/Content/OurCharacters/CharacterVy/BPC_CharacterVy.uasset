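; Player character Vy, a mage whose attack input fires a Niagara magic effect at a nearby enemy.
; Every Tick scans all BP_EnemyBase actors and stores the last one found within a short fixed radius as NearestEnemy, never clearing it.
; The attack attaches the effect to NSMageAttack, sets its end point to that enemy and plays a wand montage, with IsAttacking blocking re-entry until completion.
; No damage is applied here.
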(event `self.ReceiveBeginPlay`
  (set `self.IsAttacking?` false))

(event `EnhancedInput|/Game/OurCharacters/IA/IA_Attack`
  (params (ActionValue :type Boolean) (ElapsedSeconds :type "Float (double-precision)") (TriggeredSeconds :type "Float (double-precision)") (InputAction :type "InputAction Object Reference" :default "/Game/OurCharacters/IA/IA_Attack.IA_Attack"))
  (:`Triggered`
    (if (not (`self.IsAttacking?`))
      (set `self.IsAttacking?` true)
      (`self.PlayAnimAttack`))))

(event `self.ReceiveTick`
  (params (DeltaSeconds :type "Float (single-precision)"))
  (`self.GetNearestEnemy`))

(event `PlayAnimAttack`
  (if (`self.IsAttacking?`)
    (bind _nearestenemy (`self.NearestEnemy`)
      (:`then`
        (bind _returnvalue (`NiagaraFunctionLibrary.SpawnSystemAttached` "/Game/Niagara/N_MageAttack.N_MageAttack" (`self.NS_MageAttack`) "None" (0.0 0.0 0.0) (struct) "KeepRelativeOffset"))
        (`NiagaraComponent.SetVariableVec3` _returnvalue "EndPosition" (`self.K2_GetActorLocation` _nearestenemy))
        (`|PlayMontage` (`self.Mesh`) "/Game/ThirdParty/ModularRPGHeroesPolyart/Animations/MagicWandStance/Attack01_MagicWandAnim_Montage.Attack01_MagicWandAnim_Montage"
          (:`OnCompleted`
            (set `self.IsAttacking?` false))))
      (:`else`
        (`KismetSystemLibrary.PrintString` "Hello")
        (set `self.IsAttacking?` false)))))

(fn `GetNearestEnemy`
  (bind _outactors (`GameplayStatics.GetAllActorsOfClass` "/Game/Actors/Enemies/BP_EnemyBase.BP_EnemyBase_C"))
  (for _array_element _outactors
    (bind _returnvalue (`KismetMathLibrary.Vector_Distance` (`self.K2_GetActorLocation` _array_element) (`self.K2_GetActorLocation` (`GameplayStatics.GetPlayerCharacter` 0))))
    (if (< _returnvalue 50.0)
      (set `self.NearestEnemy` _array_element)
      (set `self.NearestDistance` _returnvalue))))

(fn `UserConstructionScript`
  (`parent.UserConstructionScript`))