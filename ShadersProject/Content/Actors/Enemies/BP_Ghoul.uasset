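; BP_Ghoul is a ghoul enemy character that tunes stats for damage, movement speed and detection range.
; On BeginPlay it runs the parent logic, then overrides those three values, so any behavior using them lies outside this graph.
; The Tick and overlap events are disabled stubs, and the construction script only calls its parent.
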(event `self.ReceiveBeginPlay`
  (`parent.ReceiveBeginPlay`)
  (set `self.DamageAmount` 15.0)
  (set `CharacterMovementComponent.MaxWalkSpeed` 400.0 (`self.CharacterMovement`))
  (set `self.DetectionRange` 750.0))

(fn `UserConstructionScript`
  (`parent.UserConstructionScript`))