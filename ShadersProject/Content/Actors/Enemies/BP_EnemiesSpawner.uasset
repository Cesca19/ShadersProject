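; Enemy spawner actor that spawns a set number of enemies at its own location, then removes itself.
; On BeginPlay a looping timer calls SpawnEnemies at the spawn rate, spawning a random class from EnemiesTypes and incrementing a counter.
; Tick watches the counter and, once it reaches EnemiesToSpawn, clears the timer and destroys the spawner.
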(event `self.ReceiveBeginPlay`
  (`KismetSystemLibrary.K2_SetTimer` null "SpawnEnemies" (`self.SpawnRate`) true))

(event `self.ReceiveTick`
  (params (DeltaSeconds :type "Float (single-precision)"))
  (if (>= (`self.EnemiesSpawned`) (`self.EnemiesToSpawn`))
    (`KismetSystemLibrary.K2_ClearTimer` null "SpawnEnemies")
    (`self.K2_DestroyActor`)))

(fn `SpawnEnemies`
  (`|SpawnActorFromClass` (`KismetArrayLibrary.Array_Random` (`self.EnemiesTypes`)) (`KismetMathLibrary.MakeTransform` (`self.K2_GetActorLocation`)) "Undefined" "MultiplyWithRoot" null null)
  (bind _result (`/Engine/EditorBlueprintResources/StandardMacros.IncrementInt` (`self.EnemiesSpawned`))
    (:`  `
      (set `self.EnemiesSpawned` _result))))

(fn `UserConstructionScript`)