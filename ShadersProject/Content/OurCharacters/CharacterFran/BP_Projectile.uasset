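; Ice projectile in Fran's character folder that freezes enemies and damages towers.
; On first overlap it disables collision, hides its mesh and zeroes max speed, then branches by target type.
; Unfrozen enemies get paused animation, disabled movement and an ice material; after a delay the projectile restores them, applies damage and destroys itself.
; Towers take immediate damage with ice effects, while already-frozen enemies and other actors just destroy the projectile.
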(event `self.ReceiveBeginPlay`)

(event `self.Sphere.OnComponentBeginOverlap`
  (params (OverlappedComponent :type "PrimitiveComponent Object Reference") (OtherActor :type "Actor Object Reference") (OtherComp :type "PrimitiveComponent Object Reference") (OtherBodyIndex :type Integer) (bFromSweep :type Boolean) (SweepResult :type "HitResult Structure (by ref)"))
  (`self.TurnOff`)
  (bind _asbp_enemy_base (cast `/Game/Actors/Enemies/BP_EnemyBase` OtherActor)
    (:`then`
      (`/Engine/EditorBlueprintResources/StandardMacros.DoOnce` false
        (:`Completed`
          (if (not (`SkeletalMeshComponent.bPauseAnims` (`Character.Mesh` _asbp_enemy_base)))
            (`self.PauseCharater` _asbp_enemy_base)
            (`KismetSystemLibrary.Delay` 3.0)
            (`self.ReleaseCharacter`)
            (`self.K2_DestroyActor`)
            (else
              (`self.K2_DestroyActor`))))))
    (:`CastFailed`
      (bind _asbp_tower_base (cast `/Game/Actors/Towers/BP_TowerBase` OtherActor)
        (:`then`
          (`GameplayStatics.ApplyDamage` _asbp_tower_base (`self.DamageAmount`))
          (bind _returnvalue (`self.K2_GetActorLocation` _asbp_tower_base))
          (`NiagaraFunctionLibrary.SpawnSystemAtLocation` "/Game/ThirdParty/Stylized_VFX_StPack/Particles/UPDATE_1_2/P_Ice_Hit_02.P_Ice_Hit_02" _returnvalue)
          (`GameplayStatics.PlaySoundAtLocation` "/Game/Sound/video-game-magic-spell-ice-shatter-gamemaster-audio-1-1-00-01.video-game-magic-spell-ice-shatter-gamemaster-audio-1-1-00-01" _returnvalue (struct) 1.0 1.0 0.0 null null null null)
          (`self.K2_DestroyActor`))
        (:`CastFailed`
          (`self.K2_DestroyActor`))))))

(fn `PauseCharater`
  (params (Enemy :type "/Game/Actors/Enemies/BP_EnemyBase Object Reference"))
  (bind _returnvalue (`self.K2_GetActorLocation` Enemy))
  (bind _mesh (`Character.Mesh` Enemy))
  (set `self.Enemy` Enemy)
  (set `SkeletalMeshComponent.bPauseAnims` true (`Character.Mesh` Enemy))
  (`CharacterMovementComponent.DisableMovement` (`Character.CharacterMovement` Enemy))
  (set `self.StartMaterial` (`PrimitiveComponent.GetMaterial` _mesh 0))
  (`PrimitiveComponent.SetMaterial` _mesh 0 "/Game/Materials/Enemy/MI_Ice.MI_Ice")
  (`NiagaraFunctionLibrary.SpawnSystemAtLocation` "/Game/ThirdParty/Stylized_VFX_StPack/Particles/UPDATE_1_2/P_Ice_Hit_02.P_Ice_Hit_02" _returnvalue)
  (`GameplayStatics.PlaySoundAtLocation` "/Game/Sound/video-game-magic-spell-ice-shatter-gamemaster-audio-1-1-00-01.video-game-magic-spell-ice-shatter-gamemaster-audio-1-1-00-01" _returnvalue (struct) 1.0 1.0 0.0 null null null null))

(fn `ReleaseCharacter`
  (bind _enemy (`self.Enemy`))
  (bind _mesh (`Character.Mesh` _enemy))
  (set `SkeletalMeshComponent.bPauseAnims` false _mesh)
  (`CharacterMovementComponent.SetMovementMode` (`Character.CharacterMovement` _enemy) "MOVE_Walking" 0)
  (`PrimitiveComponent.SetMaterial` _mesh 0 (`self.StartMaterial`))
  (`GameplayStatics.ApplyDamage` _enemy (`self.DamageAmount`)))

(fn `TurnOff`
  (`PrimitiveComponent.SetCollisionEnabled` (`self.Sphere`) "NoCollision")
  (`SceneComponent.SetVisibility` (`self.StaticMesh`) false true)
  (set `ProjectileMovementComponent.MaxSpeed` 0.0 (`self.ProjectileMovement`))
  (`KismetSystemLibrary.PrintString` "Hit"))

(fn `UserConstructionScript`)