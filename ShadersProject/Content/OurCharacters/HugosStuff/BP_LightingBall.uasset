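; Lightning ball actor that throws electric arcs onto nearby surfaces in random directions.
; On Tick, once a cooldown elapses, it line traces on Visibility along a random unit vector between a minimum and maximum radius.
; Each blocking hit spawns an attached, auto-destroying Niagara arc, fed an actor-relative start offset, a world-space end nudged off the surface, and the impact normal.
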(event `self.ReceiveTick`
  (params (DeltaSeconds :type "Float (single-precision)"))
  (`self.UpdateTrace`))

(fn `UpdateTrace`
  (locals (ImpactOffset :type "Float (double-precision)" :default 1.0))
  (bind _returnvalue (`self.K2_GetActorLocation`))
  (bind _returnvalue_2 (* (`self.Random dir`) (`self.MinRadius`)))
  ;[1 1 1] Check Cooldown
  (if (>= (- (`GameplayStatics.GetTimeSeconds`) (`self.LastTrace`)) (`self.TraceCooldown`))
    ;[1 1 1] Trace
    (set `self.Random dir` (`KismetMathLibrary.RandomUnitVector`))
    (bind _outhit (`KismetSystemLibrary.LineTraceSingle` :`Start` (+ _returnvalue _returnvalue_2) :`End` (+ _returnvalue (* (`self.Random dir`) (`self.MaxRadius`))) :`TraceChannel` "TraceTypeQuery1" :`DrawTime` (`self.TraceCooldown`)))
    ;[1 1 1] Reset Cooldown
    (set `self.LastTrace` (`GameplayStatics.GetTimeSeconds`))
    (bind (_bblockinghit _binitialoverlap _time _distance _location _impactpoint _normal _impactnormal) (`GameplayStatics.BreakHitResult` _outhit))
    ;[1 1 1] Spawn niagara
    (if _bblockinghit
      (bind _returnvalue_3 (`NiagaraFunctionLibrary.SpawnSystemAttached` "/Game/OurCharacters/HugosStuff/NS_LightingArcs.NS_LightingArcs" (`self.DefaultSceneRoot`) "None" (0.0 0.0 0.0) (struct) "KeepRelativeOffset" true))
      (`NiagaraComponent.SetVariableVec3` _returnvalue_3 "BeamStartPoint" _returnvalue_2)
      (`NiagaraComponent.SetVariableVec3` _returnvalue_3 "BeamEndPoint" (+ (* (`local.ImpactOffset`) _impactnormal) _impactpoint))
      (`NiagaraComponent.SetVariableVec3` _returnvalue_3 "ImpactNormal" _impactnormal))))

(fn `UserConstructionScript`)