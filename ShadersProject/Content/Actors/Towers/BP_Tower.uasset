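; BP_Tower is a tower actor that displays its damage state through its mesh materials.
; On BeginPlay it creates dynamic instances of the world and tech materials in the first two mesh slots.
; The OnHealthChange override calls the parent, then writes the lost-health fraction to a damage parameter on each instance.
; It also enables player input so the B key applies damage to itself, apparently for testing.
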(event `self.ReceiveBeginPlay`
  (bind _mesh (`self.Mesh`))
  (`parent.ReceiveBeginPlay`)
  (bind _returnvalue (`PrimitiveComponent.CreateDynamicMaterialInstance` _mesh 0 (`PrimitiveComponent.GetMaterial` _mesh 0) "None"))
  (set `self.MI_World` _returnvalue)
  (bind _returnvalue_2 (`PrimitiveComponent.CreateDynamicMaterialInstance` (`self.Mesh`) 1 (`PrimitiveComponent.GetMaterial` (`self.Mesh`) 1) "None"))
  (set `self.MI_Tech` _returnvalue_2)
  (`self.EnableInput` (`GameplayStatics.GetPlayerController` 0)))

(event `self.ReceiveActorBeginOverlap`
  (params (OtherActor :type "Actor Object Reference"))
  (`parent.ReceiveActorBeginOverlap` OtherActor))

(event `Key|B`
  (params (Key :type "Key Structure"))
  (:`Pressed`
    (`GameplayStatics.ApplyDamage` self 10.0)))

(fn `OnHealthChange`
  (params (NewHealth :type Integer) (MaxHealth :type Integer))
  (bind _returnvalue (`KismetMathLibrary.Conv_IntToDouble` MaxHealth))
  (bind _returnvalue_2 (/ (- _returnvalue (`KismetMathLibrary.Conv_IntToDouble` NewHealth)) _returnvalue))
  (`parent.OnHealthChange` NewHealth MaxHealth)
  (`MaterialInstanceDynamic.SetScalarParameterValue` (`self.MI_World`) "DamagePercentage" _returnvalue_2)
  (`MaterialInstanceDynamic.SetScalarParameterValue` (`self.MI_Tech`) "DamageAmount" _returnvalue_2))

(fn `UserConstructionScript`
  (`parent.UserConstructionScript`))