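; Character Blueprint for Hugo, a playable character with a double-sword attack and a teleport skill.
; IA_Shoot plays the attack montage with an attached Niagara spin effect, locked until the montage completes.
; IA_Skill checks a timestamp cooldown, spawns distortion, offsets the player forward without sweep, and drives dissolve through a timeline and material parameter collection.
; A thunder-beam effect targeting enemies in range exists but is disconnected.
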(event `self.ReceiveBeginPlay`
  (`parent.ReceiveBeginPlay`)
  (set `self.IsAttacking?` false)
  (`self.EnableInput` (`GameplayStatics.GetPlayerController` 0)))

(event `EnhancedInput|/Game/OurCharacters/IA/IA_Shoot`
  (params (ActionValue :type Boolean) (ElapsedSeconds :type "Float (double-precision)") (TriggeredSeconds :type "Float (double-precision)") (InputAction :type "InputAction Object Reference" :default "/Game/OurCharacters/IA/IA_Shoot.IA_Shoot"))
  (:`Triggered`
    (if (not (`self.IsAttacking?`))
      (set `self.IsAttacking?` true)
      (`self.PlayAttack`))))

(event `PlayAttack`
  (if (`self.IsAttacking?`)
    (`self.SpawnAttackEffect`)
    (`|PlayMontage` (`self.Mesh`) "/Game/ThirdParty/ModularRPGHeroesPolyart/Animations/DoubleSwordStance/AM_DoubleSwordAttack.AM_DoubleSwordAttack"
      (:`OnCompleted`
        (set `self.IsAttacking?` false)))))

(event `EnhancedInput|/Game/OurCharacters/IA/IA_Skill`
  (params (ActionValue :type Boolean) (ElapsedSeconds :type "Float (double-precision)") (TriggeredSeconds :type "Float (double-precision)") (InputAction :type "InputAction Object Reference" :default "/Game/OurCharacters/IA/IA_Skill.IA_Skill"))
  (:`Triggered`
    ;[1 1 1] Check Cooldown
    (if (>= (- (`GameplayStatics.GetTimeSeconds`) (`self.Last Trace`)) (`self.Cooldown`))
      (`|ExecutionSequence`
        (:`then_0`
          (`NiagaraFunctionLibrary.SpawnSystemAttached` "/Game/HugosStuff/NS/NS_Distortion.NS_Distortion" (`self.NS_Teleport`) "None" (0.0 0.0 0.0) (struct) "KeepRelativeOffset" true)
          (`self.Teleport`)
          ;[1 1 1] Reset Cooldown
          (set `self.Last Trace` (`GameplayStatics.GetTimeSeconds`))
          (`KismetSystemLibrary.Delay` 0.2)
          (`Timeline|Timeline_0` :!via `Stop`))
        (:`then_1`
          (bind (_direction _dissolve) (`Timeline|Dissolve timeline`)
            (:`Update`
              (`KismetMaterialLibrary.SetScalarParameterValue` "/Game/HugosStuff/Materials/MPC_Dissolve.MPC_Dissolve" "Dissolve" _dissolve))))))))

(fn `GetEnemyInRange`
  (params (Range :type "Float (double-precision)"))
  (returns (NearEnemy :type "Array of /Game/Actors/Enemies/BP_EnemyBase Object Reference"))
  (locals (EnemyList :type "Array of /Game/Actors/Enemies/BP_EnemyBase Object Reference"))
  (bind _enemylist (`local.EnemyList`))
  (bind _outactors (`GameplayStatics.GetAllActorsOfClass` "/Game/Actors/Enemies/BP_EnemyBase.BP_EnemyBase_C"))
  (for _array_element _outactors
    (bind _valid (`self.Is Valid Distance` _array_element Range))
    (if _valid
      (`KismetArrayLibrary.Array_Add` _enemylist _array_element)))
  (return _enemylist))

(fn `SpawnAttackEffect`
  (`NiagaraFunctionLibrary.SpawnSystemAttached` "/Game/HugosStuff/NS/NS_SpinAttack.NS_SpinAttack" (`self.NS_ElectricSword`) "None" (`self.K2_GetActorLocation` (`GameplayStatics.GetPlayerCharacter` 0)) (struct) "KeepRelativeOffset"))

(fn `Teleport`
  (bind _returnvalue (`GameplayStatics.GetPlayerCharacter` 0))
  ;[1 1 1] Teleport
  (`SceneComponent.K2_AddRelativeLocation` (`Actor.RootComponent` _returnvalue) (* (`self.GetActorForwardVector` _returnvalue) (`self.Tp range`)) false false))

(fn `UserConstructionScript`
  (`parent.UserConstructionScript`))