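; Playable character Fran, whose shoot input deploys a temporary shield instead of firing a projectile.
; Shoot sets a short wind-up timer to StartAttack, which attaches BP_Shield as a runtime child actor component if CanAttack allows, then schedules StopAttack after ShieldDuration.
; StopAttack destroys the shield and re-enables attacking, and also runs on despawn.
; The Skill function is only a debug print.
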(event `self.ReceiveBeginPlay`
  (`parent.ReceiveBeginPlay`))

(event `EnhancedInput|/Game/OurCharacters/IA/IA_Shoot`
  (params (ActionValue :type Boolean) (ElapsedSeconds :type "Float (double-precision)") (TriggeredSeconds :type "Float (double-precision)") (InputAction :type "InputAction Object Reference" :default "/Game/OurCharacters/IA/IA_Shoot.IA_Shoot"))
  (:`Triggered`
    (`self.Shoot`)))

(fn `LaunchShield`
  (if (`self.CanAttack`)
    (bind _returnvalue (`AddComponent|NODE_AddChildActorComponent-2`))
    (bind _output_get (set `self.Shield` _returnvalue))
    (`ChildActorComponent.SetChildActorClass` _output_get "/Game/OurCharacters/CharacterFran/BP_Shield.BP_Shield_C")
    (set `self.CanAttack` false)))

(fn `OnDespawn`
  (`parent.OnDespawn`)
  (`self.StopAttack`))

(fn `Shoot`
  (set `self.IsShooting` true)
  (`KismetSystemLibrary.K2_SetTimer` null "StartAttack" 1.0 false 0.05))

(fn `Skill`
  (`KismetSystemLibrary.PrintString` "Shoot"))

(fn `StartAttack`
  (bind _shieldduration (`self.ShieldDuration`))
  (`KismetSystemLibrary.K2_ClearTimer` null "StartAttack")
  (set `self.IsShooting` false)
  (`self.LaunchShield`)
  (`KismetSystemLibrary.K2_SetTimer` null "StopAttack" _shieldduration false _shieldduration))

(fn `StopAttack`
  (bind _shield (`self.Shield`))
  (`KismetSystemLibrary.K2_ClearTimer` null "StopAttack")
  (`/Engine/EditorBlueprintResources/StandardMacros.IsValid` _shield
    (:`Is Valid`
      (`ActorComponent.K2_DestroyComponent` _shield)
      (set `self.CanAttack` true)
      (set `self.IsShooting` false))))

(fn `UserConstructionScript`
  (`parent.UserConstructionScript`))