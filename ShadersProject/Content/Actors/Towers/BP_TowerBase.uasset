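; BP_TowerBase is a tower actor, named as a base, that shows its health on a widget-based health bar.
; On BeginPlay it caches the WBP_HealthBar from its widget component and seeds it with the health component's current and maximum health.
; Health change events from BPC_HealthComponent update the bar, while depletion only prints a "Dead" debug message.
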(event `self.ReceiveBeginPlay`
  (bind _bpc_healthcomponent (`self.BPC_HealthComponent`))
  (bind _aswbp_health_bar (cast `/Game/UMG/WBP_HealthBar` (`WidgetComponent.GetUserWidgetObject` (`self.HealthBar`))))
  (bind _output_get (set `self.WBP Health Bar` _aswbp_health_bar))
  (set `/Game/UMG/WBP_HealthBar.Health` (`/Game/Components/BPC_HealthComponent.Health` _bpc_healthcomponent) _output_get)
  (set `/Game/UMG/WBP_HealthBar.MaxHealth` (`/Game/Components/BPC_HealthComponent.MaxHealth` _bpc_healthcomponent) _output_get))

(event `self.BPC_HealthComponent.OnHealthChange`
  (params (NewHealth :type Integer) (MaxHealth :type Integer))
  (set `/Game/UMG/WBP_HealthBar.Health` NewHealth (`self.WBP Health Bar`)))

(event `self.BPC_HealthComponent.OnHealthDepleted`
  (`KismetSystemLibrary.PrintString` "Dead"))

(fn `UserConstructionScript`)