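; Base enemy actor that heads for the nearest tower and diverts to chase and attack the player.
; BeginPlay binds the health bar, caches the player and towers, then starts an AI move to the tower FindTower picks.
; Tick checks player distance to start chasing or stop attacking; reaching attack range starts a looping damage timer.
; Health component events update the bar and, on depletion, flag death and set a short lifespan.
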(event `self.ReceiveBeginPlay`
  (bind _bpc_healthcomponent (`self.BPC_HealthComponent`))
  (`|ExecutionSequence`
    (:`then_0`
      (bind _aswbp_health_bar (cast `/Game/UMG/WBP_HealthBar` (`WidgetComponent.GetUserWidgetObject` (`self.HealthBar`))))
      (bind _output_get (set `self.WBP Health Bar` _aswbp_health_bar))
      (set `/Game/UMG/WBP_HealthBar.Health` (`/Game/Components/BPC_HealthComponent.Health` _bpc_healthcomponent) _output_get)
      (set `/Game/UMG/WBP_HealthBar.MaxHealth` (`/Game/Components/BPC_HealthComponent.MaxHealth` _bpc_healthcomponent) _output_get))
    (:`then_1`
      (bind _asbpc_character_base (cast `/Game/OurCharacters/BPC_CharacterBase` (`GameplayStatics.GetPlayerPawn` 0)))
      (set `self.PlayerBase` _asbpc_character_base)
      (bind _outactors (`GameplayStatics.GetAllActorsOfClass` "/Game/Actors/Towers/BP_TowerBase.BP_TowerBase_C"))
      (set `self.TowerArray` _outactors)
      (bind _targettower1 (`self.FindTower`))
      (set `self.CurrentTower` _targettower1)
      (`|AIMoveTo` self (`self.K2_GetActorLocation` _targettower1) _targettower1 200.0 true))))

(event `FindGoal`
  (bind _targettower1 (`self.FindTower`))
  (bind _output_get (set `self.CurrentTower` _targettower1))
  (`|AIMoveTo` self (`self.K2_GetActorLocation` _output_get) _output_get 200.0))

(event `self.BPC_HealthComponent.OnHealthDepleted`
  (set `self.IsDead` true)
  (`self.SetLifeSpan` 0.5))

(event `self.BPC_HealthComponent.OnHealthChange`
  (params (NewHealth :type Integer) (MaxHealth :type Integer))
  (set `/Game/UMG/WBP_HealthBar.Health` NewHealth (`self.WBP Health Bar`)))

(event `self.ReceiveTick`
  (params (DeltaSeconds :type "Float (single-precision)"))
  (`/Engine/EditorBlueprintResources/StandardMacros.IsValid` (`self.PlayerBase`)
    (:`Is Valid`
      _)
    (:`Is Not Valid`
      (bind _asbpc_character_base (cast `/Game/OurCharacters/BPC_CharacterBase` (`GameplayStatics.GetPlayerPawn` 0)))
      (set `self.PlayerBase` _asbpc_character_base)))
  (if (not (<= (`self.DistanceToPlayer`) (`self.AttackRange`)))
    (`self.StopAttack`))
  (if (and (<= (`self.DistanceToPlayer`) (`self.DetectionRange`)) (not (`self.IsChasing`)) (not (`self.IsAttacking`)))
    (`self.ChasingPlayer`)))

(event `ChasingPlayer`
  (bind _playerbase (`self.PlayerBase`))
  (set `self.IsChasing` true)
  (bind _movementresult (`|AIMoveTo` self (`self.K2_GetActorLocation` _playerbase) _playerbase 0.5 true)
    (:`OnSuccess`
      (if (`|EnumEquality` _movementresult "Success")
        (set `self.IsChasing` false)
        (if (<= (`self.DistanceToPlayer`) (`self.AttackRange`))
          (`self.StartAttack`))))))

(fn `Attack`
  (`GameplayStatics.ApplyDamage` (`self.PlayerBase`) (`self.DamageAmount`) null self))

(fn `DistanceToPlayer`
  (returns (ReturnValue :type "Float (double-precision)"))
  (bind _playerbase (`self.PlayerBase`))
  (`/Engine/EditorBlueprintResources/StandardMacros.IsValid` _playerbase
    (:`Is Valid`
      (return (`KismetMathLibrary.Abs` (`KismetMathLibrary.Vector_Distance` (`self.K2_GetActorLocation` _playerbase) (`self.K2_GetActorLocation`)))))))

(fn `FindTower`
  (returns (TargetTower1 :type "/Game/Actors/Towers/BP_TowerBase Object Reference"))
  (locals (StartDistance :type "Float (double-precision)" :default 10000000.0) (TargetTower :type "/Game/Actors/Towers/BP_TowerBase Object Reference"))
  (for _array_element (`self.TowerArray`)
    (`/Engine/EditorBlueprintResources/StandardMacros.IsValid` _array_element
      (:`Is Valid`
        (bind _returnvalue (`KismetMathLibrary.Vector_Distance` (`self.K2_GetActorLocation` _array_element) (`self.K2_GetActorLocation`)))
        (if (<= _returnvalue (`local.StartDistance`))
          (set `local.StartDistance` _returnvalue)
          (set `local.TargetTower` _array_element)))))
  (return (`local.TargetTower`)))

(fn `StartAttack`
  (set `self.IsAttacking` true)
  (`KismetSystemLibrary.K2_SetTimer` null "Attack" (`self.AttackRate`) true))

(fn `StopAttack`
  (set `self.IsChasing` false)
  (set `self.IsAttacking` false)
  (`KismetSystemLibrary.K2_ClearTimer` null "Attack"))

(fn `UserConstructionScript`)